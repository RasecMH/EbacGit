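; BP_Pickup is a pickup actor with empty Body, CollisionBody and InteractionBody events that act as extension hooks.
; Sphere overlap registers it as the third-person character's last interact object, enables interaction and sets the character's look-at target, with end overlap clearing both flags.
; Interact, when allowed, runs InteractionBody and destroys the actor.
; A self-repeating delayed RotationLoop spins the mesh, though nothing here starts it.
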(event OnComponentBeginOverlap(Sphere)
  (params (OverlappedComponent :type Primitive%20Component%20Object%20Reference) (OtherActor :type Actor%20Object%20Reference) (OtherComp :type Primitive%20Component%20Object%20Reference) (OtherBodyIndex :type Integer) (bFromSweep :type Boolean) (SweepResult :type Hit%20Result%20Structure%20%28by%20ref%29))
  ;[0.15 0.15 0.15 0.5] Collision Logic
  (bind _asbp_third_person_character (Utilities|Casting|CastToBP_ThirdPersonCharacter OtherActor))
  (Variables|/Game/ThirdPerson/Blueprints/BP_ThirdPersonCharacter.BP_ThirdPersonCharacter_C|SetLastInteractObject _asbp_third_person_character self)
  (Variables|Default|SetCanInteract true)
  (CallFunction|CollisionBody)
  (Variables|/Game/ThirdPerson/Blueprints/BP_ThirdPersonCharacter.BP_ThirdPersonCharacter_C|SetIsLookAt _asbp_third_person_character true)
  (Variables|/Game/ThirdPerson/Blueprints/BP_ThirdPersonCharacter.BP_ThirdPersonCharacter_C|SetLookAtPosition _asbp_third_person_character (Transformation|GetActorLocation)))

(event OnComponentEndOverlap(Sphere)
  (params (OverlappedComponent :type Primitive%20Component%20Object%20Reference) (OtherActor :type Actor%20Object%20Reference) (OtherComp :type Primitive%20Component%20Object%20Reference) (OtherBodyIndex :type Integer))
  ;[0.15 0.15 0.15 0.5] Collision Logic
  (bind _asbp_third_person_character (Utilities|Casting|CastToBP_ThirdPersonCharacter OtherActor))
  (Variables|Default|SetCanInteract false)
  (Variables|/Game/ThirdPerson/Blueprints/BP_ThirdPersonCharacter.BP_ThirdPersonCharacter_C|SetIsLookAt _asbp_third_person_character false))

(event Custom|RotationLoop
  ;[0.15 0.15 0.15 0.5] Rotation Loop
  (Transformation|AddLocalRotation (Variables|Default|GetStaticMesh) "10.000000,10.000000,0.000000" false false)
  (Utilities|FlowControl|Delay 0.2)
  (CallFunction|RotationLoop))

(event Custom|Body)

(event Custom|CollisionBody)

(event Custom|InteractionBody)

(event EventInteract
  ;[0.15 0.15 0.15 0.5] Interact Logic
  (if (Variables|Default|GetCanInteract)
    (Variables|Default|SetCanInteract false)
    (CallFunction|InteractionBody)
    (Actor|DestroyActor)))

(event EventBeginPlay
  (CallFunction|Body))

(fn ConstructionScript)