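; BP_Enemy is an enemy character with data-driven stats and a health bar widget.
; The construction script reads the Enemy_01 row of DT_EnemyStatus, storing health and damage in Stats and writing ReactionTime to the Blackboard.
; BeginPlay caches the widget component's W_HealthBar.
; The Damage override calls the parent logic, then sets the bar from the returned value, assuming a fixed maximum of 100.
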(event EventBeginPlay
  (bind _asw_health_bar (Utilities|Casting|CastToW_HealthBar (UserInterface|GetWidget (Variables|Default|GetWidget))))
  (Variables|Default|SetCurrentHUD _asw_health_bar))

(fn ConstructionScript
  (bind _returnvalue (Utilities|GetDataTableRow "/Game/Blueprints/DataTables/DT_EnemyStatus.DT_EnemyStatus" "Enemy_01")
    (:then
      (Variables|Default|SetStats (Utilities|Struct|MakeS_Stats (.health _returnvalue) (.damage _returnvalue)))
      (AI|Components|Blackboard|SetValueasFloat (AI|GetBlackboard 0) (Utilities|Name|MakeLiteralName "ReactionTime") (.reactiontime _returnvalue)))))

(fn Damage
  (params (DamageValue :type Float%20%28double-precision%29))
  (bind _newhealth (|CallParentFunction DamageValue))
  (Progress|SetPercent (Variables|/Game/HUD/W_HealthBar.W_HealthBar_C|GetHealthBar (Variables|Default|GetCurrentHUD)) (/ _newhealth 1e+02))
  (return _newhealth))