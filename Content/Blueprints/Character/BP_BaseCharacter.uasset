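; BP_BaseCharacter is a base character Blueprint that provides simple attack and damage handling through a Stats struct.
; AttackBox overlap events track a single target, storing any overlapping BP_BaseCharacter and clearing it when that actor leaves.
; Attack damages the stored target by Stats.AttackDamage if it carries the given tag.
; Damage subtracts the value from Stats.Health and returns the new health, with no clamping or death handling.
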(event OnComponentBeginOverlap(AttackBox)
  (params (OverlappedComponent :type Primitive%20Component%20Object%20Reference) (OtherActor :type Actor%20Object%20Reference) (OtherComp :type Primitive%20Component%20Object%20Reference) (OtherBodyIndex :type Integer) (bFromSweep :type Boolean) (SweepResult :type Hit%20Result%20Structure%20%28by%20ref%29))
  (bind _asbp_base_character (Utilities|Casting|CastToBP_BaseCharacter OtherActor))
  (Variables|Default|SetOtherActor _asbp_base_character))

(event OnComponentEndOverlap(AttackBox)
  (params (OverlappedComponent :type Primitive%20Component%20Object%20Reference) (OtherActor :type Actor%20Object%20Reference) (OtherComp :type Primitive%20Component%20Object%20Reference) (OtherBodyIndex :type Integer))
  (if (== OtherActor (Variables|Default|GetOtherActor))
    (Variables|Default|SetOtherActor 0)))

(fn ConstructionScript)

(fn Damage
  (params (DamageValue :type Float%20%28double-precision%29))
  (bind _structout (Utilities|Struct|SetmembersinS_Stats (Variables|Default|GetStats) (- (.health (Variables|Default|GetStats)) DamageValue)))
  (return (.health _structout)))

(fn Attack
  (params (Tag :type Name))
  (bind _otheractor (Variables|Default|GetOtherActor))
  (Utilities|IsValid _otheractor
    (:Is%20Valid
      (if (Actor|ActorHasTag _otheractor Tag)
        (CallFunction|Damage (Variables|Default|GetOtherActor) (.attackdamage (Variables|Default|GetStats)))))))